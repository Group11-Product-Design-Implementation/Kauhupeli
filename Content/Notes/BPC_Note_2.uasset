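; Readable note Blueprint that the player picks up to view on screen and lays down again.
; The Interactable event drives a FlipFlop that alternates the two states, each playing a paper sound at the note.
; Picking up hides the Note component, shows a newly created Notes_Widget1 and blocks look and move input.
; Laying down restores visibility and input and calls LayNoteDown on that widget.
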(event EventInteractable
  (bind _returnvalue (Game|GetPlayerController 0))
  (bind _note (Variables|Default|Getnote))
  (bind _note_2 (Variables|Default|Getnote))
  (bind _returnvalue_2 (Transformation|GetWorldLocation _note))
  (Utilities|FlowControl|FlipFlop
    (:A
      (Audio|PlaySoundatLocation "/Game/Notes/Paper_Cue.Paper_Cue" _returnvalue_2 "0, 0, 0" 1.0 1.0 0.0 0 0 0 0)
      (bind _returnvalue_3 (UserInterface|CreateWidget "/Game/Notes/Notes_Widget1.Notes_Widget1_C"))
      (Rendering|SetVisibility _note_2 false false)
      (UserInterface|Viewport|AddtoViewport _returnvalue_3 0)
      (Input|SetIgnoreLookInput _returnvalue true)
      (Input|SetIgnoreMoveInput _returnvalue true))
    (:B
      (Audio|PlaySoundatLocation "/Game/Notes/Paper_Cue.Paper_Cue" _returnvalue_2 "0, 0, 0" 1.0 1.0 0.0 0 0 0 0)
      (Rendering|SetVisibility _note_2 true false)
      (Default|LayNoteDown _returnvalue_3)
      (Input|SetIgnoreLookInput _returnvalue false)
      (Input|SetIgnoreMoveInput _returnvalue false))))

(fn ConstructionScript)