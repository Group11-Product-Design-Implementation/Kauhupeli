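; Interactable note actor that the player picks up to read and lays back down.
; A FlipFlop on Interactable alternates between reading and putting down, playing a paper sound each time and toggling the note mesh's visibility.
; Reading creates the Notes widget and blocks look and move input; putting down calls LayNoteDown on the widget and restores input.
; The first read also updates the first-person character's mission through a DoOnce.
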(event EventBeginPlay
  (bind _asbp_first_person_character (Utilities|Casting|CastToBP_FirstPersonCharacter (Game|GetPlayerCharacter 0)))
  (Variables|Default|SetAs%20BP%20First%20Person%20Character _asbp_first_person_character))

(event EventInteractable
  (bind _returnvalue (Game|GetPlayerController 0))
  (bind _note (Variables|Default|Getnote))
  (bind _note_2 (Variables|Default|Getnote))
  (bind _returnvalue_2 (Transformation|GetWorldLocation _note))
  (Utilities|FlowControl|FlipFlop
    (:A
      (Audio|PlaySoundatLocation "/Game/Notes/Paper_Cue.Paper_Cue" _returnvalue_2 "0, 0, 0" 1.0 1.0 0.0 0 0 0 0)
      (bind _returnvalue_3 (UserInterface|CreateWidget "/Game/Notes/Notes_Widget.Notes_Widget_C"))
      (Rendering|SetVisibility _note_2 false false)
      (UserInterface|Viewport|AddtoViewport _returnvalue_3 0)
      (Input|SetIgnoreLookInput _returnvalue true)
      (Input|SetIgnoreMoveInput _returnvalue true)
      (bind _asbp_first_person_character (Utilities|Casting|CastToBP_FirstPersonCharacter (Variables|Default|GetAs%20BP%20First%20Person%20Character)))
      (Utilities|FlowControl|DoOnce false
        (:Completed
          (Default|UpdateMission _asbp_first_person_character (Variables|Default|GetNew%20Mission%20Set)))))
    (:B
      (Audio|PlaySoundatLocation "/Game/Notes/Paper_Cue.Paper_Cue" _returnvalue_2 "0, 0, 0" 1.0 1.0 0.0 0 0 0 0)
      (Rendering|SetVisibility _note_2 true false)
      (Default|LayNoteDown _returnvalue_3)
      (Input|SetIgnoreLookInput _returnvalue false)
      (Input|SetIgnoreMoveInput _returnvalue false))))

(event Input|MouseEvents|LeftMouseButton
  (params (Key :type Key%20Structure :default "None")))

(fn ConstructionScript)