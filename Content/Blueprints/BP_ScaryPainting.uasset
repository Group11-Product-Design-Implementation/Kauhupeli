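; Scary painting actor that plays a collapse sound and rocks on its pitch axis when any actor overlaps it.
; Tick drives an integer state machine that uses FInterpTo to swing the pitch one way, the other, then back to level, zeroing yaw and roll.
; Ending the overlap resets the state, re-arming the scare.
; An older play-once version of the logic remains in the graph but never runs.
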(event EventBeginPlay
  (Variables|Default|SetRotationState 0))

(event Collision|EventActorBeginOverlap
  (params (OtherActor :type Actor%20Object%20Reference))
  (Variables|Default|SetPlayerInRange true))

(event EventTick
  (params (DeltaSeconds :type Float%20%28single-precision%29))
  (Variables|Default|SetFrameTime DeltaSeconds)
  (if (== (Variables|Default|GetRotationState) 0)
    (if (Variables|Default|GetPlayerInRange)
      (Audio|PlaySoundatLocation "/Game/StarterContent/Audio/Collapse01.Collapse01" (Transformation|GetActorLocation) "0, 0, 0" 1.0 1.0 0.0 0 0 0 0)
      (Variables|Default|SetTargetRotation 1e+01)
      (Variables|Default|SetRotationState 1))
    (elif (== (Variables|Default|GetRotationState) 4)
      (Variables|Default|SetRotationState 3)
      (Transformation|SetActorRotation (Math|Rotator|MakeRotator 0.0 (Math|Interpolation|FInterpTo (.Pitch (Math|Rotator|BreakRotator (Transformation|GetActorRotation))) (Variables|Default|GetTargetRotation) (Variables|Default|GetFrameTime) 15.0) 0.0) :!label _label)
      (if (Math|Float|NearlyEqual(Float) (Variables|Default|GetTargetRotation) (.Pitch (Math|Rotator|BreakRotator (Transformation|GetActorRotation))) 0.05)
        (if (== (Variables|Default|GetRotationState) 1)
          (Variables|Default|SetRotationState 2)
          (Variables|Default|SetTargetRotation -1e+01)
          (elif (== (Variables|Default|GetRotationState) 2)
            (Variables|Default|SetRotationState 3)
            (Variables|Default|SetTargetRotation 0.0)
            (elif (== (Variables|Default|GetRotationState) 3)
              (Variables|Default|SetRotationState 4)))))
      (elif (== (Variables|Default|GetRotationState) 1)
        (goto _label)
        (elif (== (Variables|Default|GetRotationState) 2)
          (goto _label)
          (elif (== (Variables|Default|GetRotationState) 3)
            (goto _label)))))))

(event Collision|EventActorEndOverlap
  (params (OtherActor :type Actor%20Object%20Reference))
  (Variables|Default|SetPlayerInRange false)
  (Variables|Default|SetRotationState 0))

(fn ConstructionScript)