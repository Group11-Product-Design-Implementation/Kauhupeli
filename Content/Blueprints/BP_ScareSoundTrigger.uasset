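; BP_ScareSoundTrigger is a trigger actor that randomly plays a scare sound when another actor overlaps it.
; On begin overlap it rolls a random integer up to ChanceOfNotPlaying and spawns the sound at its own location only on zero, keeping the audio component.
; On end overlap it stops that component after a configurable delay if it is still valid.
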(event EventBeginPlay)

(event Collision|EventActorBeginOverlap
  (params (OtherActor :type Actor%20Object%20Reference))
  (if (== (Math|Random|RandomIntegerinRange 0 (Variables|Default|GetChanceOfNotPlaying)) 0)
    (bind _returnvalue (Audio|SpawnSoundatLocation (Variables|Default|GetSoundFIle) (Transformation|GetActorLocation) "0, 0, 0" 1.0 1.0 0.0 0 0))
    (Variables|Default|SetSoundRef _returnvalue)))

(event EventTick
  (params (DeltaSeconds :type Float%20%28single-precision%29)))

(event Collision|EventActorEndOverlap
  (params (OtherActor :type Actor%20Object%20Reference))
  (bind _soundref (Variables|Default|GetSoundRef))
  (if (Utilities|IsValid _soundref)
    (Audio|Components|Audio|StopDelayed _soundref (Variables|Default|GetAudioStopDelay))))

(fn ConstructionScript)