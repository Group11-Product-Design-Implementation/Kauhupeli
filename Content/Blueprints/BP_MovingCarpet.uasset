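; BP_MovingCarpet is a moving platform actor that shuttles between its placed location and a second point offset by OtherPositionDiff.
; BeginPlay caches both endpoints, and each actor overlap, with no filter on the other actor, flips the target between them, even mid-move.
; Once triggered, Tick moves it toward the current target with VInterpToConstant at MovementSpeed and sets its location without sweeping.
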(event EventBeginPlay
  (bind _returnvalue (Transformation|GetActorLocation))
  (Variables|Default|SetStartPosition1 _returnvalue)
  (Variables|Default|SetIsTargetStartPosition1 true)
  (bind _output_get (Variables|Default|SetCurrentPosition _returnvalue))
  (Variables|Default|SetStartPosition2 (+ _output_get (Variables|Default|GetOtherPositionDiff))))

(event Collision|EventActorBeginOverlap
  (params (OtherActor :type Actor%20Object%20Reference))
  (if (Variables|Default|GetIsTargetStartPosition1)
    (Variables|Default|SetTargetPosition (Variables|Default|GetStartPosition2))
    (Variables|Default|SetIsTargetStartPosition1 false)
    (else
      (Variables|Default|SetTargetPosition (Variables|Default|GetStartPosition1))
      (Variables|Default|SetIsTargetStartPosition1 true)))
  (Variables|Default|SetIsMoving true))

(event EventTick
  (params (DeltaSeconds :type Float%20%28single-precision%29))
  (Variables|Default|SetFrameTime DeltaSeconds)
  (if (Variables|Default|GetIsMoving)
    (bind _output_get (Variables|Default|SetCurrentPosition (Math|Interpolation|VInterptoConstant (Variables|Default|GetCurrentPosition) (Variables|Default|GetTargetPosition) (Variables|Default|GetFrameTime) (Variables|Default|GetMovementSpeed))))
    (Transformation|SetActorLocation _output_get false false)))

(fn ConstructionScript)