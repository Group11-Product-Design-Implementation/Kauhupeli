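; Drawer furniture actor that lets the player slide open or close whichever tagged drawer mesh they are looking at.
; Interactable line-traces from the first-person camera and stores the hit "drawer" component.
; Its relative Y position decides direction, then a timeline lerps it along local Y with an open or close sound.
; CanOpen blocks repeat triggers until the timeline ends or a fallback delay resets it.
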(event EventBeginPlay
  (Input|EnableInput (Game|GetPlayerController 0)))

(event EventInteractable
  (bind _returnvalue (Transformation|GetActorLocation))
  (Utilities|FlowControl|Sequence
    (:then_0
      (if (Variables|Default|GetCanOpen?)
        (Variables|Default|SetCanOpen? false)
        (bind _asbp_first_person_character (Utilities|Casting|CastToBP_FirstPersonCharacter (Game|GetPlayerCharacter 0)))
        (bind (_outhit _returnvalue_2) (Collision|LineTraceForObjects (Transformation|GetWorldLocation (Variables|/Game/FirstPerson/Blueprints/BP_FirstPersonCharacter.BP_FirstPersonCharacter_C|GetFirstPersonCamera _asbp_first_person_character)) (+ (Transformation|GetWorldLocation (Variables|/Game/FirstPerson/Blueprints/BP_FirstPersonCharacter.BP_FirstPersonCharacter_C|GetFirstPersonCamera _asbp_first_person_character)) (* (Math|Vector|GetForwardVector (Variables|/Game/FirstPerson/Blueprints/BP_FirstPersonCharacter.BP_FirstPersonCharacter_C|GetFirstPersonCamera _asbp_first_person_character)) 2e+02)) (Utilities|Array|MakeArray "ObjectTypeQuery2") true 0 "Persistent" false))
        (if _returnvalue_2
          (if (Components|ComponentHasTag (.HitComponent (Collision|BreakHitResult _outhit)) "drawer")
            (bind _asstatic_mesh_component (Utilities|Casting|CastToStaticMeshComponent (.HitComponent (Collision|BreakHitResult _outhit))))
            (Variables|Default|SetStatic%20Mesh%20REF _asstatic_mesh_component)
            (if (not (<= (.y (Variables|/Script/Engine.SceneComponent|GetRelativeLocation _asstatic_mesh_component)) -4e+01))
              (Audio|PlaySoundatLocation "/Game/CustomAssets/Drawer/open-drawer-85791.open-drawer-85791" _returnvalue "0, 0, 0" 1.0 1.0 0.0 0 0 0 0)
              (Variables|Default|SetStart%20Location (Math|Vector|MakeVector (.x (Variables|/Script/Engine.SceneComponent|GetRelativeLocation (Variables|Default|GetStatic%20Mesh%20REF))) (.y (Variables|/Script/Engine.SceneComponent|GetRelativeLocation (Variables|Default|GetStatic%20Mesh%20REF))) (.z (Variables|/Script/Engine.SceneComponent|GetRelativeLocation (Variables|Default|GetStatic%20Mesh%20REF)))))
              (Variables|Default|SetEnd%20Location (Math|Vector|MakeVector (.x (Variables|/Script/Engine.SceneComponent|GetRelativeLocation (Variables|Default|GetStatic%20Mesh%20REF))) (+ (.y (Variables|/Script/Engine.SceneComponent|GetRelativeLocation (Variables|Default|GetStatic%20Mesh%20REF))) -4e+01) (.z (Variables|/Script/Engine.SceneComponent|GetRelativeLocation (Variables|Default|GetStatic%20Mesh%20REF)))))
              (bind _open_drawer (Timeline|Open%20Drawer PlayFromStart)
                (:Update
                  (Transformation|SetRelativeLocation (Variables|Default|GetStatic%20Mesh%20REF) (Math|Vector|Lerp(Vector) (Variables|Default|GetStart%20Location) (Variables|Default|GetEnd%20Location) _open_drawer) false false))
                (:Finished
                  (Variables|Default|SetCanOpen? true)))
              (else
                (Audio|PlaySoundatLocation "/Game/CustomAssets/Drawer/Drawer_Close.Drawer_Close" _returnvalue "0, 0, 0" 1.0 1.0 0.0 0 0 0 0)
                (Variables|Default|SetStart%20Location (Math|Vector|MakeVector (.x (Variables|/Script/Engine.SceneComponent|GetRelativeLocation (Variables|Default|GetStatic%20Mesh%20REF))) (.y (Variables|/Script/Engine.SceneComponent|GetRelativeLocation (Variables|Default|GetStatic%20Mesh%20REF))) (.z (Variables|/Script/Engine.SceneComponent|GetRelativeLocation (Variables|Default|GetStatic%20Mesh%20REF)))))
                (Variables|Default|SetEnd%20Location (Math|Vector|MakeVector (.x (Variables|/Script/Engine.SceneComponent|GetRelativeLocation (Variables|Default|GetStatic%20Mesh%20REF))) (+ (.y (Variables|/Script/Engine.SceneComponent|GetRelativeLocation (Variables|Default|GetStatic%20Mesh%20REF))) 4e+01) (.z (Variables|/Script/Engine.SceneComponent|GetRelativeLocation (Variables|Default|GetStatic%20Mesh%20REF)))))
                (bind _open_drawer_2 (Timeline|Timeline PlayFromStart)
                  (:Update
                    (Transformation|SetRelativeLocation (Variables|Default|GetStatic%20Mesh%20REF) (Math|Vector|Lerp(Vector) (Variables|Default|GetStart%20Location) (Variables|Default|GetEnd%20Location) _open_drawer_2) false false))
                  (:Finished
                    (Variables|Default|SetCanOpen? true)))))))))
    (:then_1
      (Utilities|FlowControl|Delay 0.8)
      (Variables|Default|SetCanOpen? true))))

(fn ConstructionScript)