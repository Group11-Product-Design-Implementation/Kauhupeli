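; BPC_Key is a key pickup that gives the first-person player character a key and updates their mission.
; BeginPlay caches the player character, and the Interactable event sets its Haskey flag, plays a rustle sound at the key and destroys the actor.
; After the DestroyActor call, the same event passes NewMissionSet to the character's UpdateMission through a DoOnce gate.
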(event EventBeginPlay
  (bind _asbp_first_person_character (Utilities|Casting|CastToBP_FirstPersonCharacter (Game|GetPlayerCharacter 0)))
  (Variables|Default|SetAs%20BP%20First%20Person%20Character_0 _asbp_first_person_character))

(event EventInteractable
  (Variables|/Game/FirstPerson/Blueprints/BP_FirstPersonCharacter.BP_FirstPersonCharacter_C|SetHaskey? (stale EventBeginPlay _asbp_first_person_character) true)
  (Audio|PlaySoundatLocation "/Game/Mission_Triggers/Key/Key_rustle_Sound.Key_rustle_Sound" (Transformation|GetWorldLocation (Variables|Default|Getkey1)) "0, 0, 0" 1.0 1.0 0.0 0 0 0 0)
  (Actor|DestroyActor)
  (bind _asbp_first_person_character (Utilities|Casting|CastToBP_FirstPersonCharacter (Variables|Default|GetAs%20BP%20First%20Person%20Character_0)))
  (Utilities|FlowControl|DoOnce false
    (:Completed
      (Default|UpdateMission _asbp_first_person_character (Variables|Default|GetNewMissionSet)))))

(fn ConstructionScript)